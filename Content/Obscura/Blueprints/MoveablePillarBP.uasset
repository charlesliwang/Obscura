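; MoveablePillarBP is a pillar that shifts along the world Y axis with the player's movement while pillar mode is active.
; Each Tick looks up the first ObscuraCharacter and CompassManager, then writes the manager's InPillarRange from the player's distance to the pillar.
; When in range with PillarMode on, it adds scaled player Y velocity to the pillar's position, without sweep or delta-time scaling.
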(event `self.ReceiveTick`
  (params (DeltaSeconds :type "Float (single-precision)"))
  (bind _outactors (`GameplayStatics.GetAllActorsOfClass` "/Script/Obscura.ObscuraCharacter"))
  (bind _outactors_2 (`GameplayStatics.GetAllActorsOfClass` "/Game/Obscura/Blueprints/CompassManager.CompassManager_C"))
  (bind _item (`KismetArrayLibrary.Array_Get` _outactors))
  (bind _output_get (set `Compass.inPillarRange` (< (`KismetMathLibrary.VSize` (- (`self.K2_GetActorLocation` _item) (`SceneComponent.K2_GetComponentLocation` (`self.Pillar`)))) 1500.0) (`KismetArrayLibrary.Array_Get` _outactors_2)))
  (if (and _output_get (`ObscuraCharacter.pillarMode` _item))
    (`SceneComponent.K2_SetWorldLocation` (`self.Pillar`) (`KismetMathLibrary.MakeVector` (.x (`SceneComponent.K2_GetComponentLocation` (`self.Pillar`))) (+ (.y (`SceneComponent.K2_GetComponentLocation` (`self.Pillar`))) (* (.y (`self.GetVelocity` _item)) 0.025)) (.z (`SceneComponent.K2_GetComponentLocation` (`self.Pillar`)))) false false)))

(fn `UserConstructionScript`)